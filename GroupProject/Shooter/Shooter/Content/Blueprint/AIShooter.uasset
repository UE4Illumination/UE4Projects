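; AI enemy pawn that wanders, chases any Shooter it sees, and is destroyed when its health runs out.
; While the Success flag is true, Tick issues a new AI move to a random nearby reachable point every frame.
; PawnSensing clears the flag to chase a seen Shooter; reaching it restores wandering, while a failed move leaves it off.
; TakeDamage subtracts from Health and destroys the actor at zero or below.
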(event `self.ReceiveBeginPlay`)

(event `self.ReceiveActorBeginOverlap`
  (params (OtherActor :type "Actor Object Reference")))

(event `self.ReceiveTick`
  (params (DeltaSeconds :type "Float (single-precision)"))
  (if (`self.Success`)
    (`|AIMoveTo` self (`NavigationSystem.GetRandomReachablePointInRadius` (`self.K2_GetActorLocation`) 1000.0)
      (:`OnSuccess`
        (set `self.Success` true))
      (:`OnFail`
        (set `self.Success` false)))))

(event `self.PawnSensing.OnSeePawn`
  (params (Pawn :type "Pawn Object Reference"))
  (bind _asshooter (cast `/Game/Blueprint/Shooter` Pawn)
    (:`then`
      (set `self.Success` false)
      (`|AIMoveTo` self (0.0 0.0 0.0) _asshooter
        (:`OnSuccess`
          (set `self.Success` true))
        (:`OnFail`
          (set `self.Success` false))))
    (:`CastFailed`
      (set `self.Success` true))))

(fn `TakeDamage`
  (params (DMG :type "Float (double-precision)"))
  (set `self.Health` (- (`self.Health`) DMG))
  (if (<= (`self.Health`) 0.0)
    (`self.K2_DestroyActor`)))

(fn `UserConstructionScript`)