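; Player-controlled shooter character with walking, sprinting, clamped look pitch and a HUD created at begin play.
; Jump velocity differs between moving and standing.
; Holding Shoot counts down an attack timer using Tick's delta time, then line-traces from above the actor toward the camera's aim point and damages any AIShooter hit.
; Shots consume clip ammo, and Reload, manual or on firing empty, refills it from the reserve.
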(event `self.ReceiveBeginPlay`)

(event `self.ReceiveActorBeginOverlap`
  (params (OtherActor :type "Actor Object Reference")))

(event `self.ReceiveTick`
  (params (DeltaSeconds :type "Float (single-precision)"))
  (set `self.DT` DeltaSeconds))

(event `InputAxis|moveForward`
  (params (AxisValue :type "Float (single-precision)"))
  (`self.AddMovementInput` (`KismetMathLibrary.GetForwardVector` (`KismetMathLibrary.MakeRotator` 0.0 0.0 (.yaw (`self.GetControlRotation`)))) AxisValue))

(event `InputAxis|MoveSide`
  (params (AxisValue :type "Float (single-precision)"))
  (`self.AddMovementInput` (`KismetMathLibrary.GetRightVector` (`KismetMathLibrary.MakeRotator` 0.0 0.0 (.yaw (`self.GetControlRotation`)))) AxisValue))

(event `InputAxis|Turn`
  (params (AxisValue :type "Float (single-precision)"))
  (`self.AddControllerYawInput` AxisValue))

(event `InputAxis|LookUp`
  (params (AxisValue :type "Float (single-precision)"))
  (`self.AddControllerPitchInput` AxisValue)
  (`Controller.SetControlRotation` (`self.GetController`) (`KismetMathLibrary.MakeRotator` (.roll (`self.GetControlRotation`)) (`KismetMathLibrary.ClampAngle` (.pitch (`self.GetControlRotation`)) (`self.Max Look Down`) (`self.Max Look Up`)) (.yaw (`self.GetControlRotation`)))))

(event `self.ReceiveBeginPlay`
  (bind _returnvalue (`|CreateWidget` "/Game/Blueprint/Hud.Hud_C"))
  (set `self.Hud` _returnvalue)
  (`UserWidget.AddToViewport` _returnvalue 0)
  (set `CharacterMovementComponent.MaxWalkSpeed` (`self.MoveSpeed`) (`self.CharacterMovement`)))

(event `InputAction|Sprint`
  (params (Key :type "Key Structure" :default "AnyKey"))
  (:`Pressed`
    (set `CharacterMovementComponent.MaxWalkSpeed` (`self.SprintSpeed`) (`self.CharacterMovement`)))
  (:`Released`
    (set `CharacterMovementComponent.MaxWalkSpeed` (`self.MoveSpeed`) (`self.CharacterMovement`))))

(event `InputAction|Jump`
  (params (Key :type "Key Structure" :default "AnyKey"))
  (bind _charactermovement (`self.CharacterMovement`))
  (:`Pressed`
    (if (> (`KismetMathLibrary.VSize` (`MovementComponent.Velocity` (`self.CharacterMovement`))) 0.0)
      (`self.Jump`)
      (set `CharacterMovementComponent.JumpZVelocity` (`self.JumpHeightRuning`) _charactermovement)
      (else
        (`self.Jump`)
        (set `CharacterMovementComponent.JumpZVelocity` (`self.JumpHeightStanding`) _charactermovement)))))

(event `InputAxis|Shoot`
  (params (AxisValue :type "Float (single-precision)"))
  (bind _camera (`self.Camera`))
  (if (== AxisValue 1.0)
    (if (<= (`self.AttackSpeed`) 0.0)
      (set `self.AttackSpeed` (`self.MaxAttackSpeed`))
      (bind _outhit (`KismetSystemLibrary.LineTraceSingle` :`Start` (+ (`self.K2_GetActorLocation`) (* (`self.GetActorUpVector`) 70.0)) :`End` (+ (`SceneComponent.K2_GetComponentLocation` _camera) (* (`SceneComponent.GetForwardVector` _camera) (`self.Range`))) :`TraceChannel` "TraceTypeQuery1" :`DrawDebugType` "ForDuration"))
      (if (<= (`self.Ammo`) 0.0)
        (`self.Reload`)
        (else
          (set `self.Ammo` (- (`self.Ammo`) 1.0))
          (bind _asaishooter (cast `/Game/Blueprint/AIShooter` (`.HitActor` (`GameplayStatics.BreakHitResult` _outhit))))
          (`/Game/Blueprint/AIShooter.TakeDamage` _asaishooter (`self.Damage`))))
      (else
        (set `self.AttackSpeed` (- (`self.AttackSpeed`) (* (`self.AttackRate`) (`self.DT`))))))
    (else
      (set `self.AttackSpeed` (`self.MaxAttackSpeed`)))))

(event `InputAction|Reload`
  (params (Key :type "Key Structure" :default "AnyKey"))
  (:`Pressed`
    (`self.Reload`)))

(event `Reload`
  (if (< (`self.Ammo`) (`self.ClipMax`))
    (if (> (`self.MaxAmmo`) 0.0)
      (set `self.ReloadAmount` (- (`self.ClipMax`) (`self.Ammo`)))
      (if (< (`self.ReloadAmount`) (`self.MaxAmmo`))
        (set `self.Ammo` (`self.ClipMax`))
        (set `self.MaxAmmo` (- (`self.MaxAmmo`) (`self.ReloadAmount`)))
        (else
          (set `self.Ammo` (`self.MaxAmmo`))
          (set `self.MaxAmmo` 0.0))))))

(fn `UserConstructionScript`)