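; SwapMan is a player character with sprint, multi-jump, wall climbing, wall running and a position-swap ability.
; Sprinting into WallClimb or WallRun actors passes axis-aligned facing or hit-normal checks to set state flags.
; While W is held, Tick uses those flags to drive Flying movement up walls or forward with gradual descent.
; Swap line-traces from the camera and exchanges locations with a swappable SwapObjectTest; BeginPlay adds the SwapHud widget.
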(event `self.CapsuleComponent.OnComponentBeginOverlap`
  (params (OtherActor :type "Actor Object Reference") (OtherComp :type "PrimitiveComponent Object Reference") (OtherBodyIndex :type Integer) (bFromSweep :type Boolean) (SweepResult :type "HitResult Structure (by ref)"))
  (bind (_bblockinghit _binitialoverlap _time _location _impactpoint _normal) (`GameplayStatics.BreakHitResult` SweepResult))
  (bind _returnvalue (`self.GetActorForwardVector`))
  (bind _returnvalue_2 (`self.GetActorRightVector`))
  (`|ExecutionSequence`
    (:`then_0`
      (bind _aswall_climb (cast `/Game/BluePrints/WallClimb` OtherActor))
      (set `self.WallClimbVar` _aswall_climb)
      (if (or (== _returnvalue (0.0 1.0 0.0) :`ErrorTolerance` 0.1) (== _returnvalue (1.0 0.0 0.0) :`ErrorTolerance` 0.1) (== _returnvalue (0.0 -1.0 0.0) :`ErrorTolerance` 0.1) (== _returnvalue (-1.0 0.0 0.0) :`ErrorTolerance` 0.1))
        (`KismetSystemLibrary.PrintString` (`KismetStringLibrary.Conv_VectorToString` _normal))
        (`KismetSystemLibrary.PrintString` (`KismetStringLibrary.Conv_VectorToString` _returnvalue) true true (struct :`R` 1.0 :`G` 0.069946 :`B` 0.079495 :`A` 1.0))
        (if (and (not (`self.WallRun`)) (not (`self.LedgeGrab`)))
          (if (`self.SprintPress`)
            (set `CharacterMovementComponent.MaxFlySpeed` (`self.RunClimbSpeed`) (`self.CharacterMovement`))
            (set `self.WallClimb` true)))))
    (:`then_1`
      (bind _aswall_run (cast `/Game/BluePrints/WallRun` OtherActor))
      (set `self.WallRunVar` _aswall_run)
      (if (or (and (`KismetMathLibrary.InRange_FloatFloat` (.y _returnvalue_2) -0.2 0.7) (== _normal (-1.0 0.0 0.0) :`ErrorTolerance` 0.1)) (and (`KismetMathLibrary.InRange_FloatFloat` (.x (`self.GetActorRightVector`)) -1.0 1.0) (== _normal (1.0 0.0 0.0) :`ErrorTolerance` 0.1)) (and (`KismetMathLibrary.InRange_FloatFloat` (.y (`self.GetActorRightVector`)) -1.0 1.0) (== _normal (0.0 -1.0 0.0) :`ErrorTolerance` 0.1)) (and (`KismetMathLibrary.InRange_FloatFloat` (.x (`self.GetActorRightVector`)) -1.0 1.0) (== _normal (0.0 1.0 0.0) :`ErrorTolerance` 0.1)))
        (`KismetSystemLibrary.PrintString` (`KismetStringLibrary.Conv_VectorToString` _returnvalue_2) true true (struct :`R` 1.0 :`G` 0.069946 :`B` 0.079495 :`A` 1.0))
        (if (and (not (`self.WallClimb`)) (not (`self.LedgeGrab`)))
          (if (`self.SprintPress`)
            (set `CharacterMovementComponent.MaxFlySpeed` (`self.WallRunSpeed`) (`self.CharacterMovement`))
            (set `self.WallRun` true)))))))

(event `self.ReceiveBeginPlay`
  (bind _returnvalue (`|CreateWidget` "/Game/BluePrints/SwapHud.SwapHud_C" (`GameplayStatics.GetPlayerController` 0)))
  (set `self.Hud` _returnvalue)
  (`UserWidget.AddToViewport` _returnvalue 0)
  (set `CharacterMovementComponent.MaxWalkSpeed` (`self.MoveSpeed`) (`self.CharacterMovement`)))

(event `self.ReceiveActorBeginOverlap`
  (params (OtherActor :type "Actor Object Reference")))

(event `self.ReceiveTick`
  (params (DeltaSeconds :type "Float (single-precision)"))
  (set `self.DT` DeltaSeconds)
  (`|ExecutionSequence`
    (:`then_0`
      (if (`self.WallClimb`)
        (`self.WallClimbing`)))
    (:`then_1`
      (if (`self.WallRun`)
        (`self.WallRunning`)))))

(event `InputAxis|MoveForward`
  (params (AxisValue :type "Float (single-precision)"))
  (if (not (`self.StopMovement`))
    (`self.AddMovementInput` (`KismetMathLibrary.GetForwardVector` (`KismetMathLibrary.MakeRotator` 0.0 0.0 (.yaw (`self.GetControlRotation`)))) AxisValue)))

(event `InputAction|Sprint`
  (params (Key :type "Key Structure" :default "AnyKey"))
  (:`Pressed`
    (if (not (`self.StopMovement`))
      (set `CharacterMovementComponent.MaxWalkSpeed` (`self.SprintSpeed`) (`self.CharacterMovement`))
      (set `self.SprintPress` true)
      (if (`self.ShouldClimbWhenStanding?`)
        (for _array_element (`PrimitiveComponent.GetOverlappingActors` (`self.CapsuleComponent`) "/Game/BluePrints/WallClimb.WallClimb_C")
          (bind _aswall_climb (cast `/Game/BluePrints/WallClimb` _array_element))
          (set `self.WallClimbVar` _aswall_climb)
          (if (and (not (`self.WallRun`)) (not (`self.LedgeGrab`)))
            (set `CharacterMovementComponent.MaxFlySpeed` (`self.StandClimbSpeed`) (`self.CharacterMovement`))
            (set `self.WallClimb` true))))))
  (:`Released`
    (set `CharacterMovementComponent.MaxWalkSpeed` (`self.MoveSpeed`) (`self.CharacterMovement`))
    (set `self.SprintPress` false)))

(event `self.CapsuleComponent.OnComponentEndOverlap`
  (params (OtherActor :type "Actor Object Reference") (OtherComp :type "PrimitiveComponent Object Reference") (OtherBodyIndex :type Integer))
  (`|ExecutionSequence`
    (:`then_0`
      (bind _aswall_climb (cast `/Game/BluePrints/WallClimb` OtherActor))
      (set `self.WallClimbVar` _aswall_climb)
      (set `self.WallClimb` false)
      (`self.WallClimbing`))
    (:`then_1`
      (bind _aswall_run (cast `/Game/BluePrints/WallRun` OtherActor))
      (set `self.WallRunVar` _aswall_run)
      (set `self.WallRun` false)
      (`self.WallRunning`))))

(event `InputAxis|MoveSide`
  (params (AxisValue :type "Float (single-precision)"))
  (if (not (`self.StopMovement`))
    (`self.AddMovementInput` (`KismetMathLibrary.GetRightVector` (`KismetMathLibrary.MakeRotator` 0.0 0.0 (.yaw (`self.GetControlRotation`)))) AxisValue)))

(event `InputAxis|Turn`
  (params (AxisValue :type "Float (single-precision)"))
  (`self.AddControllerYawInput` AxisValue))

(event `InputAxis|lookUp`
  (params (AxisValue :type "Float (single-precision)"))
  (`self.AddControllerPitchInput` AxisValue)
  (`Controller.SetControlRotation` (`self.GetController`) (`KismetMathLibrary.MakeRotator` (.roll (`self.GetControlRotation`)) (`KismetMathLibrary.ClampAngle` (.pitch (`self.GetControlRotation`)) (`self.Max Look Down`) (`self.Max Look Up`)) (.yaw (`self.GetControlRotation`)))))

(event `InputAction|Jump`
  (params (Key :type "Key Structure" :default "AnyKey"))
  (bind _charactermovement (`self.CharacterMovement`))
  (:`Pressed`
    (if (not (`self.StopMovement`))
      (if (> (`KismetMathLibrary.VSize` (`MovementComponent.Velocity` (`self.CharacterMovement`))) 0.0)
        (`self.Jump`)
        (set `CharacterMovementComponent.JumpZVelocity` (`self.JumpHeightRuning`) _charactermovement)
        (set `self.JumpPress` true)
        (else
          (`self.Jump`)
          (set `CharacterMovementComponent.JumpZVelocity` (`self.JumpHeightStanding`) _charactermovement)
          (set `self.JumpPress` true)))
      (set `self.JumpCount` (+ (`self.JumpCount`) 1))
      (if (`NavMovementComponent.IsMovingOnGround` (`self.CharacterMovement`))
        (set `self.JumpCount` 0)
        (elif (< (`self.JumpCount`) (`self.MaxJumpCount`))
          (`CharacterMovementComponent.SetMovementMode` (`self.CharacterMovement`) "MOVE_Walking" 0)
          (`self.Jump`)
          (set `self.JumpCount` (+ (`self.JumpCount`) 1))))))
  (:`Released`
    (set `self.JumpPress` false)))

(event `InputAction|Swap`
  (params (Key :type "Key Structure" :default "AnyKey"))
  (bind _camera (`self.Camera`))
  (:`Pressed`
    (if (not (`self.CanSwap`))
      (bind _outhit (`KismetSystemLibrary.LineTraceSingle` :`Start` (`SceneComponent.K2_GetComponentLocation` _camera) :`End` (+ (* (`KismetMathLibrary.GetForwardVector` (`SceneComponent.K2_GetComponentRotation` _camera)) (`self.SwapRange`)) (`SceneComponent.K2_GetComponentLocation` (`self.Camera`))) :`TraceChannel` "TraceTypeQuery1" :`DrawDebugType` "ForDuration"))
      (bind _asswap_object_test (cast `/Game/BluePrints/SwapObjectTest` (`.HitActor` (`GameplayStatics.BreakHitResult` _outhit))))
      (if (`/Game/BluePrints/SwapObjectTest.Swap` _asswap_object_test)
        (set `self.SwapVector` (`self.K2_GetActorLocation` _asswap_object_test))
        (`self.K2_SetActorLocation` _asswap_object_test (`self.K2_GetActorLocation`) false true)
        (`self.K2_SetActorLocation` (`self.SwapVector`) false true)))))

(fn `UserConstructionScript`)

(fn `WallClimbing`
  (if (`PlayerController.IsInputKeyDown` (`GameplayStatics.GetPlayerController` 0) "W")
    (if (`self.WallClimb`)
      (`CharacterMovementComponent.SetMovementMode` (`self.CharacterMovement`) "MOVE_Flying" 0)
      (`self.AddMovementInput` (`self.GetActorUpVector`))
      (else
        (`CharacterMovementComponent.SetMovementMode` (`self.CharacterMovement`) "MOVE_Falling" 0)))
    (else
      (`CharacterMovementComponent.SetMovementMode` (`self.CharacterMovement`) "MOVE_Walking" 0))))

(fn `WallRunning`
  (if (`PlayerController.IsInputKeyDown` (`GameplayStatics.GetPlayerController` 0) "W")
    (if (`self.WallRun`)
      (`CharacterMovementComponent.SetMovementMode` (`self.CharacterMovement`) "MOVE_Flying" 0)
      (`self.AddMovementInput` (`self.GetActorForwardVector`) 1.0)
      (`self.K2_SetActorLocation` (+ (`self.K2_GetActorLocation`) (* (`self.GetActorUpVector`) (* (`self.WallRunFallRate`) (`self.DT`) -1.0))) true)
      (else
        (`CharacterMovementComponent.SetMovementMode` (`self.CharacterMovement`) "MOVE_Falling" 0)))
    (else
      (`CharacterMovementComponent.SetMovementMode` (`self.CharacterMovement`) "MOVE_Falling" 0))))